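; Game instance for a platformer that handles level changes behind a screen transition.
; On Init it creates one UI_Transition widget, which its TransitionIn and TransitionOut functions add to the viewport if needed and play.
; OpenLevelName and OpenLevelRef events play the transition in, wait a fixed delay, then open the level by name or object reference.
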(event `self.ReceiveInit`
  (bind _returnvalue (`|CreateWidget` "/Game/UI/UI_Transition.UI_Transition_C"))
  (set `self.UITransition` _returnvalue))

(event `OpenLevelName`
  (params (LevelName :type Name))
  (`self.TransitionIn`)
  (`KismetSystemLibrary.Delay` 1.5)
  (`GameplayStatics.OpenLevel` LevelName))

(event `OpenLevelRef`
  (params (Level :type "World Soft Object Reference"))
  (`self.TransitionIn`)
  (`KismetSystemLibrary.Delay` 1.5)
  (`GameplayStatics.OpenLevelBySoftObjectPtr` Level))

(fn `TransitionIn`
  (if (not (`Widget.IsInViewport` (`self.UITransition`)))
    (`UserWidget.AddToViewport` (`self.UITransition`) 0))
  (`/Game/UI/UI_Transition.Trans In` (`self.UITransition`)))

(fn `TransitionOut`
  (if (not (`Widget.IsInViewport` (`self.UITransition`)))
    (`UserWidget.AddToViewport` (`self.UITransition`) 0))
  (`/Game/UI/UI_Transition.Trans Out` (`self.UITransition`)))