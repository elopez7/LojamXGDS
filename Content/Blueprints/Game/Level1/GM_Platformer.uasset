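; GM_Platformer is the Level 1 platformer game mode, with logic for building a vertical stack of BP_Tile blocks.
; AddBlock spawns each tile at a fixed Z spacing from the LastBlock counter, then increments it.
; CurrentEnvironment sets the tile's overlap box collision, query-only for Volkano and off for Normal and Flying.
; BeginPlay is empty, and the loop that would fill up to AmountOfBlocks is disconnected.
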(event `self.ReceiveBeginPlay`)

(fn `AddBlock`
  (bind _returnvalue (`|SpawnActorFromClass` "/Game/Blueprints/Game/Actors/BP_Tile.BP_Tile_C" (`KismetMathLibrary.MakeTransform` (`KismetMathLibrary.MakeVector` 0.0 0.0 (* (`self.LastBlock`) 2000.0))) "Undefined" "MultiplyWithRoot" null null))
  (`/Engine/EditorBlueprintResources/StandardMacros.IncrementInt` (`self.LastBlock`)
    (:`  `
      (switch `/Game/Blueprints/Enums/E_CurrentEnvironment` (`self.CurrentEnvironment`)
        (:`NewEnumerator0`
          (bind _overlapbox (`/Game/Blueprints/Game/Actors/BP_Tile.OverlapBox` _returnvalue))
          (`PrimitiveComponent.SetCollisionEnabled` _overlapbox "NoCollision"))
        (:`NewEnumerator1`
          (`PrimitiveComponent.SetCollisionEnabled` _overlapbox "QueryOnly"))
        (:`NewEnumerator2`
          (`PrimitiveComponent.SetCollisionEnabled` _overlapbox "NoCollision"))))))

(fn `UserConstructionScript`)