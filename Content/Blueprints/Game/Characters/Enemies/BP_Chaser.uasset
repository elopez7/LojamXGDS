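; BP_Chaser is an enemy character that acquires the player as a chase target when they enter its AggroRange.
; The first player overlap hands that pawn to its AIC_Chaser controller as TargetPawn, gated by a DoOnce with no reset.
; A MoveTowards event applies movement input and snaps the actor between two opposite rotations based on the sign of the direction's X.
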(event `self.AggroRange.OnComponentBeginOverlap`
  (params (OverlappedComponent :type "PrimitiveComponent Object Reference") (OtherActor :type "Actor Object Reference") (OtherComp :type "PrimitiveComponent Object Reference") (OtherBodyIndex :type Integer) (bFromSweep :type Boolean) (SweepResult :type "HitResult Structure (by ref)"))
  (bind _asbp_player (cast `/Game/Blueprints/Game/Characters/Player/BP_Player` OtherActor))
  (`/Engine/EditorBlueprintResources/StandardMacros.DoOnce` false
    (:`Completed`
      (bind _asaic_chaser (cast `/Game/Blueprints/Game/AI/AIC_Chaser` (`AIBlueprintHelperLibrary.GetAIController` self)))
      (set `/Game/Blueprints/Game/AI/AIC_Chaser.TargetPawn` _asbp_player _asaic_chaser))))

(event `MoveTowards`
  (params (WorldDirection :type "Vector Structure") (ScaleValue :type "Float (single-precision)" :default 1.0))
  (`self.AddMovementInput` WorldDirection ScaleValue)
  (`self.K2_SetActorRotation` (`KismetMathLibrary.SelectRotator` (struct) (struct :`Yaw` 180.0) (< (.x WorldDirection) 0.0))))

(fn `UserConstructionScript`
  (`parent.UserConstructionScript`))