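; BP_Tile is a platformer level tile that randomizes its layout and requests the next block as the player progresses.
; On BeginPlay, SpawnObstacles makes a weighted roll per preplaced platform mesh, toggling visibility and collision rather than spawning actors.
; The center, bottom-center and top-center pieces are weighted to always appear.
; When BP_Player enters OverlapBox, the tile calls AddBlock on GM_Platformer, then destroys itself after a short delay.
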(event `self.ReceiveBeginPlay`
  (`self.SpawnObstacles`))

(event `self.OverlapBox.OnComponentBeginOverlap`
  (params (OverlappedComponent :type "PrimitiveComponent Object Reference") (OtherActor :type "Actor Object Reference") (OtherComp :type "PrimitiveComponent Object Reference") (OtherBodyIndex :type Integer) (bFromSweep :type Boolean) (SweepResult :type "HitResult Structure (by ref)"))
  (cast `/Game/Blueprints/Game/Characters/Player/BP_Player` OtherActor)
  (bind _asgm_platformer (cast `/Game/Blueprints/Game/Level1/GM_Platformer` (`GameplayStatics.GetGameMode`)))
  (`/Game/Blueprints/Game/Level1/GM_Platformer.AddBlock` _asgm_platformer)
  (`KismetSystemLibrary.Delay` 2.0)
  (`self.K2_DestroyActor`))

(fn `SetPlatformVisible`
  (params (Mesh :type "StaticMeshComponent Object Reference") (SpawnChances :type "Float (double-precision)"))
  (if (`KismetMathLibrary.RandomBoolWithWeight` SpawnChances)
    (`SceneComponent.SetVisibility` Mesh true true)
    (`PrimitiveComponent.SetCollisionEnabled` Mesh "QueryAndPhysics")
    (else
      (`SceneComponent.SetVisibility` Mesh false false)
      (`PrimitiveComponent.SetCollisionEnabled` Mesh "NoCollision"))))

(fn `SpawnObstacles`
  (`|ExecutionSequence`
    (:`then_0`
      (`self.SetPlatformVisible` (`self.Platform1`) 0.7))
    (:`then_1`
      (`self.SetPlatformVisible` (`self.CenterPlatform`) 1.0))
    (:`then_2`
      (`self.SetPlatformVisible` (`self.BottomCenter`) 1.0))
    (:`then_3`
      (`self.SetPlatformVisible` (`self.Platform5`) 0.7))
    (:`then_4`
      (`self.SetPlatformVisible` (`self.Platform11`) 0.7))
    (:`then_5`
      (`self.SetPlatformVisible` (`self.Platform12`) 0.7))
    (:`then_6`
      (`self.SetPlatformVisible` (`self.Platform13`) 0.7))
    (:`then_7`
      (`self.SetPlatformVisible` (`self.TopRight`) 0.7))
    (:`then_8`
      (`self.SetPlatformVisible` (`self.Platform16`) 0.8))
    (:`then_9`
      (`self.SetPlatformVisible` (`self.TopCenter`) 8.0))
    (:`then_10`
      (`self.SetPlatformVisible` (`self.Platform18`) 0.7))
    (:`then_11`
      (`self.SetPlatformVisible` (`self.Platform19`) 0.7))
    (:`then_12`
      (`self.SetPlatformVisible` (`self.Platform20`) 0.7))
    (:`then_13`
      (`self.SetPlatformVisible` (`self.TopLeft`) 0.7))
    (:`then_14`
      (`self.SetPlatformVisible` (`self.Platform8`) 0.7))
    (:`then_15`
      (`self.SetPlatformVisible` (`self.Platform9`) 0.7))
    (:`then_16`
      (`self.SetPlatformVisible` (`self.Platform10`) 0.7))
    (:`then_17`
      (`self.SetPlatformVisible` (`self.Platform15`) 0.7))))

(fn `UserConstructionScript`)