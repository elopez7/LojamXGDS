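; Platform tile actor, apparently a menu variant of the platformer's level tile, with its gameplay logic disconnected.
; SwitchPlatformMesh runs SpawnObstacles, which gives each platform a random rock or steam mesh for Volkano or Flying mode through SetPlatformVisible.
; The controller reference and event binding sit in unwired nodes, so the IsValid check guards an unset variable.
; Chaser spawning, block counting with self-destruction, lethal walls and random platform visibility are also unwired.
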(event `self.ReceiveBeginPlay`)

(event `SwitchPlatformMesh`
  (params (NewMovementMode :type "EMovementMode Enum" :default "MOVE_None"))
  (`self.SpawnObstacles`))

(event `self.OverlapBox.OnComponentBeginOverlap`
  (params (OverlappedComponent :type "PrimitiveComponent Object Reference") (OtherActor :type "Actor Object Reference") (OtherComp :type "PrimitiveComponent Object Reference") (OtherBodyIndex :type Integer) (bFromSweep :type Boolean) (SweepResult :type "HitResult Structure (by ref)")))

(event `self.Wall.OnComponentBeginOverlap`
  (params (OverlappedComponent :type "PrimitiveComponent Object Reference") (OtherActor :type "Actor Object Reference") (OtherComp :type "PrimitiveComponent Object Reference") (OtherBodyIndex :type Integer) (bFromSweep :type Boolean) (SweepResult :type "HitResult Structure (by ref)")))

(event `self.Wall1.OnComponentBeginOverlap`
  (params (OverlappedComponent :type "PrimitiveComponent Object Reference") (OtherActor :type "Actor Object Reference") (OtherComp :type "PrimitiveComponent Object Reference") (OtherBodyIndex :type Integer) (bFromSweep :type Boolean) (SweepResult :type "HitResult Structure (by ref)")))

(fn `SetPlatformVisible`
  (params (InMesh :type "StaticMeshComponent Object Reference"))
  (`/Engine/EditorBlueprintResources/StandardMacros.IsValid` (`self.As GC Platformer`)
    (:`Is Valid`
      (switch `/Game/Blueprints/Enums/E_CurrentEnvironment` (`/Game/Blueprints/Game/Level1/GC_Platformer.MovementMove` (`self.As GC Platformer`))
        (:`NewEnumerator1`
          (`StaticMeshComponent.SetStaticMesh` (`local.InMesh`) (`KismetArrayLibrary.Array_Random` (`self.RockPlatforms`))))
        (:`NewEnumerator2`
          (`StaticMeshComponent.SetStaticMesh` (`local.InMesh`) (`KismetArrayLibrary.Array_Random` (`self.SteamPlatforms`))))))))

(fn `SpawnObstacles`
  (`|ExecutionSequence`
    (:`then_0`
      (`self.SetPlatformVisible` (`self.Platform1`)))
    (:`then_1`
      (`self.SetPlatformVisible` (`self.CenterPlatform`)))
    (:`then_2`
      (`self.SetPlatformVisible` (`self.BottomCenter`)))
    (:`then_3`
      (`self.SetPlatformVisible` (`self.Platform5`)))
    (:`then_4`
      (`self.SetPlatformVisible` (`self.Platform11`)))
    (:`then_5`
      (`self.SetPlatformVisible` (`self.Platform12`)))
    (:`then_6`
      (`self.SetPlatformVisible` (`self.Platform13`)))
    (:`then_7`
      (`self.SetPlatformVisible` (`self.TopRight`)))
    (:`then_8`
      (`self.SetPlatformVisible` (`self.Platform16`)))
    (:`then_9`
      (`self.SetPlatformVisible` (`self.TopCenter`)))
    (:`then_10`
      (`self.SetPlatformVisible` (`self.Platform18`)))
    (:`then_11`
      (`self.SetPlatformVisible` (`self.Platform19`)))
    (:`then_12`
      (`self.SetPlatformVisible` (`self.Platform20`)))
    (:`then_13`
      (`self.SetPlatformVisible` (`self.TopLeft`)))
    (:`then_14`
      (`self.SetPlatformVisible` (`self.Platform8`)))
    (:`then_15`
      (`self.SetPlatformVisible` (`self.Platform9`)))
    (:`then_16`
      (`self.SetPlatformVisible` (`self.Platform10`)))
    (:`then_17`
      (`self.SetPlatformVisible` (`self.Platform15`)))
    (:`then_18`
      (`self.SetPlatformVisible` (`self.Platform21`)))))

(fn `UserConstructionScript`)