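; BPC_Health is a component that tracks an actor's health and defeated state.
; On BeginPlay it sets current health to the maximum.
; ReceiveDamage subtracts the damage, clamps the result between zero and max health, and flags IsDefeated when health reaches zero.
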(event `self.ReceiveBeginPlay`
  (set `self.CurrentHealth` (`self.MaxHealth`)))

(fn `ReceiveDamage`
  (params (DamageAmount :type "Float (double-precision)"))
  (bind _output_get (set `self.CurrentHealth` (`KismetMathLibrary.FClamp` (- (`self.CurrentHealth`) (`local.DamageAmount`)) 0.0 (`self.MaxHealth`))))
  (if (<= _output_get 0.0)
    (set `self.IsDefeated` true)))